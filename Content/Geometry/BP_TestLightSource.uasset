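; BP_TestLightSource is a test actor that draws a laser beam between two positionable endpoints.
; Construction script and BeginPlay both run Initialize, which flattens the two position variables to Z=0 and applies them as relative locations to DirectionA and DirectionB.
; Initialize then calls FocusBeam to set the particle beam's source and end from SourceA and SourceB, before rotating the Direction components to face each other.
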(event `self.ReceiveBeginPlay`
  (`self.Initialize`))

(fn `FocusBeam`
  (`ParticleSystemComponent.SetBeamSourcePoint` (`self.LaserC`) 0 (`SceneComponent.K2_GetComponentLocation` (`self.SourceA`)) 0)
  (`ParticleSystemComponent.SetBeamEndPoint` (`self.LaserC`) 0 (`SceneComponent.K2_GetComponentLocation` (`self.SourceB`))))

(fn `Initialize`
  (set `self.SourceAPosition` (* (`self.SourceAPosition`) (1.0 1.0 0.0)))
  (set `self.SourceBPosition` (* (`self.SourceBPosition`) (1.0 1.0 0.0)))
  (`SceneComponent.K2_SetRelativeLocation` (`self.DirectionA`) (`self.SourceAPosition`) false false)
  (`SceneComponent.K2_SetRelativeLocation` (`self.DirectionB`) (`self.SourceBPosition`) false false)
  (`self.FocusBeam`)
  (`SceneComponent.K2_SetWorldRotation` (`self.DirectionA`) (`KismetMathLibrary.FindLookAtRotation` (`SceneComponent.K2_GetComponentLocation` (`self.DirectionA`)) (`SceneComponent.K2_GetComponentLocation` (`self.DirectionB`))) false false)
  (`SceneComponent.K2_SetWorldRotation` (`self.DirectionB`) (`KismetMathLibrary.FindLookAtRotation` (`SceneComponent.K2_GetComponentLocation` (`self.DirectionB`)) (`SceneComponent.K2_GetComponentLocation` (`self.DirectionA`))) false false))

(fn `UserConstructionScript`
  (`self.Initialize`))