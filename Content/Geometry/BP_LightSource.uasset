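; BP_LightSource is a laser light source actor with two endpoints, LaserA and LaserB, and a LaserParticle beam, but none of its logic currently runs.
; Its Construction Script and events are empty, leaving disconnected nodes that would set beam parameters and turn the endpoints toward each other.
; The LasersPointAt helper builds those transforms with a look-at rotation pitched back 90 degrees, placed at a shared Height taken from LaserBTransform.
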(fn `LasersPointAt`
  (params (Start :type "Transform Structure") (Target :type "Transform Structure"))
  (returns (NewTransform :type "Transform Structure"))
  (return (`KismetMathLibrary.MakeTransform` (`KismetMathLibrary.MakeVector` (.x Start_Location) (.y Start_Location) (`self.Height`)) (`KismetMathLibrary.MakeRotator` (.roll (`KismetMathLibrary.FindLookAtRotation` Start_Location Target_Location)) (+ (.pitch (`KismetMathLibrary.FindLookAtRotation` Start_Location Target_Location)) -90.0) (.yaw (`KismetMathLibrary.FindLookAtRotation` Start_Location Target_Location))) Start_Scale)))

(fn `UserConstructionScript`)