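; BP_GlassBlock is a colored glass block that lets a TopDownCharacter of the same color pass through and blocks other colors.
; The construction script creates a dynamic material and tints it from a color array indexed by the block's glass color (Clear, Blue or Red).
; When the collision box is overlapped, the cube's collision is switched off for an exact color match and on otherwise, with debug prints.
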(event `self.CollisionBox.OnComponentBeginOverlap`
  (params (OverlappedComponent :type "PrimitiveComponent Object Reference") (OtherActor :type "Actor Object Reference") (OtherComp :type "PrimitiveComponent Object Reference") (OtherBodyIndex :type Integer) (bFromSweep :type Boolean) (SweepResult :type "HitResult Structure (by ref)"))
  (`KismetSystemLibrary.PrintString` "Player Overlapped")
  (bind _astop_down_character (cast `/Game/TopDownCPP/Blueprints/TopDownCharacter` OtherActor)
    (:`then`
      (bind _returnvalue (select `bool` (`|EnumEquality` (`/Game/TopDownCPP/Blueprints/TopDownCharacter.CharacterColor` _astop_down_character) (`self.EGlassColor`)) :`false` (enumliteral `ECollisionEnabled` "QueryAndPhysics") :`true` (enumliteral `ECollisionEnabled` "NoCollision")))
      (`PrimitiveComponent.SetCollisionEnabled` (`self.Cube`) _returnvalue)
      (`KismetSystemLibrary.PrintString` (`|GetEnumeratorNameAsString` _returnvalue)))
    (:`CastFailed`
      (`KismetSystemLibrary.PrintString` "Cast to topdownchar failed"))))

(event `self.ReceiveActorBeginOverlap`
  (params (OtherActor :type "Actor Object Reference")))

(fn `UserConstructionScript`
  (locals (GlassMaterial :type "Material Object Reference"))
  (bind _returnvalue (`PrimitiveComponent.CreateDynamicMaterialInstance` (`self.Cube`) 0 null))
  (bind _output_get (set `self.GlassDynamicMaterial` _returnvalue))
  (`MaterialInstanceDynamic.SetVectorParameterValue` _output_get "GlassColor" (`|GetArrayItem` (`self.LCGlassColor`) (select `/Game/Geometry/EGlassColor` (`self.EGlassColor`) :`NewEnumerator1` 1 :`NewEnumerator2` 2))))