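; Reflective wall that bounces an incoming trace off its surface and collects the points along the path.
; HandleTrace records the hit point, then fires a debug-drawn object line trace along the direction mirrored about the hit normal.
; If that trace hits a BP_Emissive, it calls that actor's HandleTrace with Z-zeroed vectors and appends the returned points, chaining reflections.
; A MaxReflections check on the result length can end the trace early.
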(fn `HandleTrace`
  (params (StartingPoint :type "Vector Structure") (NormalizedDirection :type "Vector Structure") (HitNormal :type "Vector Structure") (TraceLength :type Integer) (ObjectTypes :type "Array of EObjectTypeQuery Enum (by ref)" :default _))
  (returns (Waypoints :type "Array of Vector Structure"))
  (locals (Result :type "Array of Vector Structure") (`Length of Trace` :type Integer :default 0) (ObjectTypeIgnoreList :type "Array of EObjectTypeQuery Enum"))
  (bind _result (`local.Result`))
  (`|ExecutionSequence`
    (:`then_0`
      (`KismetArrayLibrary.Array_Add` (`local.Result`) StartingPoint)
      (if (>= (`KismetArrayLibrary.Array_Length` (`local.Result`)) (`self.MaxReflections`))
        (return (`local.Result`))))
    (:`then_1`
      (set `local.Length of Trace` TraceLength))
    (:`then_2`
      (set `local.ObjectTypeIgnoreList` ObjectTypes))
    (:`then_3`
      (bind _outhit (`KismetSystemLibrary.LineTraceSingleForObjects` :`Start` StartingPoint :`End` (+ StartingPoint (* (`KismetMathLibrary.Normal` (`self.GetReflectedVector` NormalizedDirection HitNormal)) (`local.Length of Trace`))) :`ObjectTypes` (`local.ObjectTypeIgnoreList`) :`DrawDebugType` "ForDuration" :`DrawTime` 2.0))
      ;[1 1 1] Could also add cast check for BP_EmissivePawn to catch hits on enemies
      (bind _asbp_emissive (cast `/Game/Emissives/BP_Emissive` (`.HitActor` (`GameplayStatics.BreakHitResult` _outhit))))
      (bind _waypoints (`self.HandleTrace` _asbp_emissive (* (`KismetMathLibrary.SelectVector` (`.Location` (`GameplayStatics.BreakHitResult` _outhit)) (`.TraceEnd` (`GameplayStatics.BreakHitResult` _outhit)) (`GameplayStatics.BreakHitResult` _outhit)) (1.0 1.0 0.0)) (* (`KismetMathLibrary.Normal` (- (`.TraceEnd` (`GameplayStatics.BreakHitResult` _outhit)) (`.TraceStart` (`GameplayStatics.BreakHitResult` _outhit)))) (1.0 1.0 0.0)) (* (`.Normal` (`GameplayStatics.BreakHitResult` _outhit)) (1.0 1.0 0.0)) (`local.Length of Trace`) (`local.ObjectTypeIgnoreList`)))
      (`KismetArrayLibrary.Array_Append` _result _waypoints)
      (return _result))))

(fn `UserConstructionScript`)