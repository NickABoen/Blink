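; Player controller for a drag-to-blink move that sends the player pawn along a mouse-drawn direction until it hits something.
; Holding SetDestination draws a debug-line telegraph; releasing converts the screen drag into a flat world direction.
; Tick-fed gates run the telegraph and a one-shot, near-unlimited object trace, then sweep the pawn to the hit or trace end.
; The retrace gate and Emissive cast on the hit actor lead to no further logic.
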(event `Start Telegraph`
  (goto _label :!via `Open`))

(event `Stop Telegraph`
  (goto _label :!via `Close`))

(event `self.ReceiveTick`
  (params (DeltaSeconds :type "Float (single-precision)"))
  (bind _returnvalue (`self.K2_GetActorLocation` (`GameplayStatics.GetPlayerPawn` 0)))
  (`|ExecutionSequence`
    (:`then_0`
      (`/Engine/EditorBlueprintResources/StandardMacros.Gate` true :!label _label
        (:`Exit`
          (`self.DrawTelegraph` 500))))
    (:`then_1`
      (`/Engine/EditorBlueprintResources/StandardMacros.Gate` true :!label _label_2
        (:`Exit`
          (`self.Stop Trace`)
          (bind _outhit (`KismetSystemLibrary.LineTraceSingleForObjects` :`Start` _returnvalue :`End` (+ _returnvalue (`self.Direction`)) :`ObjectTypes` (`|MakeArray` "ObjectTypeQuery1" "ObjectTypeQuery2" :!type "EObjectTypeQuery Enum") :`DrawDebugType` "ForDuration" :`DrawTime` 2.0))
          (`self.K2_SetActorLocation` (`GameplayStatics.GetPlayerPawn` 0) (`KismetMathLibrary.SelectVector` (`.Location` (`GameplayStatics.BreakHitResult` _outhit)) (`.TraceEnd` (`GameplayStatics.BreakHitResult` _outhit)) (`GameplayStatics.BreakHitResult` _outhit)) true false)
          (cast `Emissive` (`.HitActor` (`GameplayStatics.BreakHitResult` _outhit))))))
    (:`then_2`
      (`/Engine/EditorBlueprintResources/StandardMacros.Gate` true :!label _label_3))))

(event `Start Trace`
  (goto _label_2 :!via `Open`))

(event `Stop Trace`
  (goto _label_2 :!via `Close`))

(event `Start Retrace`
  (goto _label_3 :!via `Open`))

(event `Stop Retrace`
  (goto _label_3 :!via `Close`))

(event `InputAction|SetDestination`
  (params (Key :type "Key Structure"))
  (bind (_locationx _locationy) (`self.GetMousePosition` (`GameplayStatics.GetPlayerController` 0)))
  (:`Pressed`
    (set `self.StartMousePress` (`KismetMathLibrary.MakeVector2D` _locationx _locationy))
    (`self.Start Telegraph`))
  (:`Released`
    (set `self.EndMousePress` (`KismetMathLibrary.MakeVector2D` _locationx _locationy))
    (`self.Stop Telegraph`)
    (set `self.Direction` (`self.ConvertMousePositionToWorldSpace` (`self.StartMousePress`) (`self.EndMousePress`) 2147483647))
    (`self.Start Trace`)))

(fn `ConvertMousePositionToWorldSpace`
  (params (`Start Position` :type "Vector2D Structure") (`End Position` :type "Vector2D Structure") (Length :type Integer))
  (returns (Result :type "Vector Structure"))
  (bind (_returnvalue_x _returnvalue_y) (`KismetMathLibrary.BreakVector2D` (* (`KismetMathLibrary.Normal2D` (- `End Position` `Start Position`)) (1.0 -1.0))))
  (return (* (`KismetMathLibrary.MakeVector` _returnvalue_y _returnvalue_x) Length)))

(fn `DrawTelegraph`
  (params (Length :type Integer))
  (bind (_locationx _locationy) (`self.GetMousePosition` (`GameplayStatics.GetPlayerController` 0)))
  (bind _returnvalue (`self.K2_GetActorLocation` (`GameplayStatics.GetPlayerPawn` 0)))
  (`KismetSystemLibrary.FlushPersistentDebugLines`)
  (`KismetSystemLibrary.DrawDebugLine` _returnvalue (+ _returnvalue (`self.ConvertMousePositionToWorldSpace` (`self.StartMousePress`) (`KismetMathLibrary.MakeVector2D` _locationx _locationy) Length)) (struct :`B` 1.0 :`A` 1.0) 0.0 3.0))

(fn `UserConstructionScript`)