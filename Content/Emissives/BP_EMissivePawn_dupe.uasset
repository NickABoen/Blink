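; Emissive pawn whose color state is Clear, Blue or Red, taking on the color of glass blocks it overlaps.
; On actor overlap it casts to BP_GlassBlock and copies that block's color enum into PlayerColor.
; The construction script maps PlayerColor to the tint of the player particles and light.
; The overlap event only stores the value and does not refresh those visuals itself.
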(event `self.ReceiveBeginPlay`)

(event `self.ReceiveActorBeginOverlap`
  (params (OtherActor :type "Actor Object Reference"))
  (bind _asbp_glass_block (cast `/Game/Geometry/BP_GlassBlock` OtherActor))
  (set `self.PlayerColor` (`/Game/Geometry/BP_GlassBlock.EGlassColor` _asbp_glass_block)))

(fn `UserConstructionScript`
  (bind _returnvalue (select `/Game/Geometry/EGlassColor` (`self.PlayerColor`) :`NewEnumerator0` (struct :`R` 1.0 :`G` 1.0 :`B` 1.0 :`A` 1.0) :`NewEnumerator1` (struct :`G` 0.312642 :`B` 1.0 :`A` 1.0) :`NewEnumerator2` (struct :`R` 1.0 :`A` 1.0) :!type "LinearColor Structure"))
  (`ParticleSystemComponent.SetColorParameter` (`self.PlayerParticles`) "InstanceColorScaleOverLife" _returnvalue)
  (`LightComponent.SetLightColor` (`self.Light`) _returnvalue true))